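; A GameInstance that manages the game's save slots and holds the currently active player save.
; On Init it loads or creates a master SaveGameData object, which serves as an index of slot names.
; LoadSaveGame loads the named SavePlayerData slot, or creates one, registers its name in the index and writes both objects to disk.
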(event `self.ReceiveInit`
  (bind _returnvalue (`GameplayStatics.DoesSaveGameExist` "SaveGameData"))
  (if _returnvalue
    (bind _returnvalue_2 (`GameplayStatics.LoadGameFromSlot` "SaveGameData"))
    (bind _assave_game_data (cast `/Game/Blueprints/Save/SaveGameData` _returnvalue_2))
    (set `self.As Save Game Data` _assave_game_data)
    (else
      (bind _returnvalue_3 (`GameplayStatics.CreateSaveGameObject` "/Game/Blueprints/Save/SaveGameData.SaveGameData_C"))
      (set `self.As Save Game Data` _returnvalue_3))))

(event `LoadSaveGame`
  (params (`Slot Name` :type String))
  (bind _returnvalue (`GameplayStatics.DoesSaveGameExist` `Slot Name`))
  (if _returnvalue
    (bind _returnvalue_2 (`GameplayStatics.LoadGameFromSlot` `Slot Name`))
    (bind _assave_player_data (cast `/Game/Blueprints/Save/SavePlayerData` _returnvalue_2))
    (bind _output_get (set `self.CurrentSaveData` _assave_player_data))
    (set `/Game/Blueprints/Save/SavePlayerData.Slot Name` `Slot Name` _output_get)
    (else
      (bind _returnvalue_3 (`GameplayStatics.CreateSaveGameObject` "/Game/Blueprints/Save/SavePlayerData.SavePlayerData_C"))
      (bind _output_get_2 (set `self.CurrentSaveData` _returnvalue_3))
      (bind _output_get_3 (set `/Game/Blueprints/Save/SavePlayerData.Slot Name` `Slot Name` _output_get_2))
      (`KismetArrayLibrary.Array_Add` (`/Game/Blueprints/Save/SaveGameData.SaveSlots` (`self.As Save Game Data`)) _output_get_3)
      (`GameplayStatics.SaveGameToSlot` (`self.As Save Game Data`) "SaveGameData")
      (`GameplayStatics.SaveGameToSlot` (`self.CurrentSaveData`) _output_get_3))))