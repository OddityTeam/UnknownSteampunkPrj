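; SavePoint is a world actor that lets the side-scroller character open a save prompt while standing near it.
; Its Sphere overlap enables input from the first player controller when the SideScrollerCharacter enters and disables it on exit.
; Pressing Z while input is enabled creates a PopUpSaveDialogue widget, passing itself as the SavePoint, and adds it to the viewport.
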(event `self.Sphere.OnComponentBeginOverlap`
  (params (OverlappedComponent :type "PrimitiveComponent Object Reference") (OtherActor :type "Actor Object Reference") (OtherComp :type "PrimitiveComponent Object Reference") (OtherBodyIndex :type Integer) (bFromSweep :type Boolean) (SweepResult :type "HitResult Structure (by ref)"))
  (cast `/Game/SideScrollerCPP/Blueprints/SideScrollerCharacter` OtherActor)
  (`self.EnableInput` (`GameplayStatics.GetPlayerController` 0)))

(event `self.Sphere.OnComponentEndOverlap`
  (params (OverlappedComponent :type "PrimitiveComponent Object Reference") (OtherActor :type "Actor Object Reference") (OtherComp :type "PrimitiveComponent Object Reference") (OtherBodyIndex :type Integer))
  (cast `/Game/SideScrollerCPP/Blueprints/SideScrollerCharacter` OtherActor)
  (`self.DisableInput` (`GameplayStatics.GetPlayerController` 0)))

(event `Key|Z`
  (params (Key :type "Key Structure"))
  (:`Pressed`
    (bind _returnvalue (`|CreateWidget` "/Game/Blueprints/UI/PopUpSaveDialogue.PopUpSaveDialogue_C" null self))
    (`UserWidget.AddToViewport` _returnvalue 0)))

(fn `UserConstructionScript`)