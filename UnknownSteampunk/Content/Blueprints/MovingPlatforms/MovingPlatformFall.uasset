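; A rotating moving platform that falls after a set delay when the side-scroller character hits it, then returns.
; BeginPlay drives the rotation through a timeline lerping between start and end rotators.
; Two timelines, meant to match, lower the platform mesh and a separate Cube, which keeps the player from rotating and falling off.
; A DoOnce reverses both timelines after the fall and is reset by each hit.
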(event `self.ReceiveHit`
  (params (MyComp :type "PrimitiveComponent Object Reference") (Other :type "Actor Object Reference") (OtherComp :type "PrimitiveComponent Object Reference") (bSelfMoved :type Boolean) (HitLocation :type "Vector Structure") (HitNormal :type "Vector Structure") (NormalImpulse :type "Vector Structure") (Hit :type "HitResult Structure (by ref)"))
  (cast `/Game/SideScrollerCPP/Blueprints/SideScrollerCharacter` Other)
  (`KismetSystemLibrary.Delay` (`self.FallAfterSetSeconds`))
  (`|ExecutionSequence`
    (:`then_0`
      ;[1 1 1] Cube Movement (so player is not rotating -> not falling off)
      ;;[1 1 1] THIS NODES MUST BE THE SAME
      (bind (_direction _fall) (`Timeline|Timeline_1` :!label _label)
        (:`Update`
          (`SceneComponent.K2_SetRelativeLocation` (`self.Cube`) (`KismetMathLibrary.MakeVector` 0.0 0.0 (.z _fall)) false false))))
    (:`then_1`
      (bind (_direction_2 _fall_2) (`Timeline|Timeline_0` :!label _label_2)
        (:`Update`
          (`SceneComponent.K2_SetRelativeLocation` (`self.Moving Platform Fall`) (`KismetMathLibrary.MakeVector` 0.0 0.0 (.z _fall_2)) false false))
        (:`Finished`
          (`/Engine/EditorBlueprintResources/StandardMacros.DoOnce` false :!label _label_3
            (:`Completed`
              (`|ExecutionSequence`
                (:`then_0`
                  (goto _label_2 :!via `Reverse`))
                (:`then_1`
                  (goto _label :!via `Reverse`))))))))
    (:`then_2`
      (goto _label_3 :!via `Reset`))))

(event `self.ReceiveBeginPlay`
  (bind (_direction _rotation_z) (`Timeline|RotationPlatform`)
    (:`Update`
      (`SceneComponent.K2_SetRelativeRotation` (`self.Moving Platform Fall`) (`KismetMathLibrary.RLerp` (`self.StartRotation`) (`self.EndRotation`) _rotation_z) false false))))

(fn `UserConstructionScript`)