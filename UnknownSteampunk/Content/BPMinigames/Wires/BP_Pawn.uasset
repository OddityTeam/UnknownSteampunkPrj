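; Player pawn for the wires minigame that lets the player drag wires with the mouse.
; On BeginPlay it switches the view to the BP_Wires actor and shows the cursor.
; Left click traces from the cursor to grab a BP_Wire, and release traces again to attach it to a valid wire or reset it.
; While a wire is held, Tick moves its end to where the mouse ray intersects the wire's plane.
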(event `self.ReceiveBeginPlay`
  (bind _returnvalue (`GameplayStatics.GetPlayerController` 0))
  (bind _outactors (`GameplayStatics.GetAllActorsOfClass` "/Game/BPMinigames/Wires/BP_Wires.BP_Wires_C"))
  (`PlayerController.SetViewTargetWithBlend` _returnvalue (`|GetArrayItem` _outactors) 0.0 "VTBlend_Linear" 0.0 false)
  (set `PlayerController.bShowMouseCursor` true _returnvalue))

(event `self.ReceiveTick`
  (params (DeltaSeconds :type "Float (single-precision)"))
  (`self.UpdateGrab`))

(event `Key|LeftMouseButton`
  (params (Key :type "Key Structure"))
  (:`Pressed`
    (`self.StartGrab`))
  (:`Released`
    (`self.EndGrab`)))

(event `StartGrab`
  (bind (_worldlocation _worlddirection) (`PlayerController.DeprojectMousePositionToWorld` (`GameplayStatics.GetPlayerController` 0)))
  (bind (_outhit _returnvalue) (`KismetSystemLibrary.LineTraceSingle` :`Start` _worldlocation :`End` (+ _worldlocation (* _worlddirection 1000.0)) :`TraceChannel` "TraceTypeQuery1" :`DrawDebugType` "ForOneFrame"))
  (if _returnvalue
    (bind (_bblockinghit _binitialoverlap _time _distance _location _impactpoint _normal _impactnormal _physmat _hitactor _hitcomponent) (`GameplayStatics.BreakHitResult` _outhit))
    (bind _asbp_wire (cast `/Game/BPMinigames/Wires/BP_Wire` _hitactor))
    (if (`/Game/BPMinigames/Wires/BP_Wire.CanGrab` _asbp_wire _hitcomponent)
      (bind _output_get (set `self.grabWire` _asbp_wire))
      (`/Game/BPMinigames/Wires/BP_Wire.StartGrab` _output_get))))

(event `EndGrab`
  (bind (_worldlocation _worlddirection) (`PlayerController.DeprojectMousePositionToWorld` (`GameplayStatics.GetPlayerController` 0)))
  (`self.grabWire`
    (:`then`
      (bind (_outhit _returnvalue) (`KismetSystemLibrary.LineTraceSingle` :`Start` _worldlocation :`End` (+ _worldlocation (* _worlddirection 1000.0)) :`TraceChannel` "TraceTypeQuery1" :`DrawDebugType` "ForOneFrame"))
      (if _returnvalue
        (bind (_bblockinghit _binitialoverlap _time _distance _location _impactpoint _normal _impactnormal _physmat _hitactor _hitcomponent) (`GameplayStatics.BreakHitResult` _outhit))
        (bind _asbp_wire (cast `/Game/BPMinigames/Wires/BP_Wire` _hitactor)
          (:`then`
            (if (`/Game/BPMinigames/Wires/BP_Wire.CanAttach` _asbp_wire _hitcomponent)
              (`/Game/BPMinigames/Wires/BP_Wire.Attach` (`self.grabWire`) _asbp_wire)
              (set `self.grabWire` null)
              (else
                (`/Game/BPMinigames/Wires/BP_Wire.Reset` (`self.grabWire`)))))
          (:`CastFailed`
            (`/Game/BPMinigames/Wires/BP_Wire.Reset` (`self.grabWire`))))))
    (:`else`)))

(event `UpdateGrab`
  (bind (_worldlocation _worlddirection) (`PlayerController.DeprojectMousePositionToWorld` (`GameplayStatics.GetPlayerController` 0)))
  (bind _grabwire (`self.grabWire`)
    (:`then`
      (bind (_t _intersection _returnvalue) (`KismetMathLibrary.LinePlaneIntersection_OriginNormal` _worldlocation (+ _worldlocation (* _worlddirection 1000.0)) (`self.K2_GetActorLocation` _grabwire) (`self.GetActorForwardVector` _grabwire)))
      (if _returnvalue
        (`/Game/BPMinigames/Wires/BP_Wire.SetEndLocation` _grabwire _intersection)
        (`KismetSystemLibrary.DrawDebugSphere` _intersection)))
    (:`else`)))

(event `ResetGrab`
  (bind _grabwire (`self.grabWire`)
    (:`then`
      (`/Game/BPMinigames/Wires/BP_Wire.Reset` _grabwire))
    (:`else`)))

(fn `UserConstructionScript`)